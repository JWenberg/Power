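; Base projectile Blueprint that shows a configurable particle effect in flight and an impact effect when it hits something.
; The construction script assigns the MovingProjectile template to the FlyingParticle component.
; On Hit, it spawns ImpactParticle at the actor's location with a configurable offset and rotation, then deactivates the flight particle.
; A short delay precedes destroying the particle component and the actor.
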(event `self.ReceiveHit`
  (params (MyComp :type "PrimitiveComponent Object Reference") (Other :type "Actor Object Reference") (OtherComp :type "PrimitiveComponent Object Reference") (bSelfMoved :type Boolean) (HitLocation :type "Vector Structure") (HitNormal :type "Vector Structure") (NormalImpulse :type "Vector Structure") (Hit :type "HitResult Structure (by ref)"))
  (`GameplayStatics.SpawnEmitterAtLocation` (`self.Impact_Particle`) (+ (`self.K2_GetActorLocation`) (`self.Location offset Impact Particle`)) (`self.Rotate_Impact_Particle`))
  (`ActorComponent.Deactivate` (`self.Flying_Particle`))
  (`KismetSystemLibrary.Delay` 2.0)
  (`ActorComponent.K2_DestroyComponent` (`self.Flying_Particle`))
  (`self.K2_DestroyActor`))

(fn `UserConstructionScript`
  (`ParticleSystemComponent.SetTemplate` (`self.Flying_Particle`) (`self.Moving_Projectile`)))