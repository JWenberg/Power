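; Base homing projectile Blueprint for powers that flies toward a target entity and shows an impact effect on reaching it.
; On BeginPlay it applies the flight particle and, after a brief delay, sets a valid target's capsule as the ProjectileMovement homing target.
; Overlapping only that target spawns the impact emitter, stops movement, then after staggered delays deactivates the trail, flags Impacted and destroys the actor.
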(event `self.ReceiveBeginPlay`
  (bind _targetentity (`self.TargetEntity`))
  (`ParticleSystemComponent.SetTemplate` (`self.Flying_Particle`) (`self.Moving_Projectile`))
  (`KismetSystemLibrary.Delay` 0.02)
  (if (`KismetSystemLibrary.IsValid` _targetentity)
    (set `ProjectileMovementComponent.HomingTargetComponent` (`Character.CapsuleComponent` _targetentity) (`self.ProjectileMovement`))))

(event `self.ReceiveActorBeginOverlap`
  (params (OtherActor :type "Actor Object Reference"))
  (if (== OtherActor (`self.TargetEntity`))
    (`GameplayStatics.SpawnEmitterAtLocation` (`self.Impact_Particle`) (`SceneComponent.K2_GetComponentLocation` (`ProjectileMovementComponent.HomingTargetComponent` (`self.ProjectileMovement`))))
    (`MovementComponent.StopMovementImmediately` (`self.ProjectileMovement`))
    (`KismetSystemLibrary.Delay` 0.1)
    (`ActorComponent.Deactivate` (`self.Flying_Particle`))
    (`KismetSystemLibrary.Delay` 0.5)
    (set `self.Impacted` true)
    (`self.K2_DestroyActor`)))

(fn `UserConstructionScript`)