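; GA_MeleeAttack is a Gameplay Ability for a melee attack that damages the entity named by a gameplay event.
; On activation it commits, waits once for Skills.MeleeAttack.DealDamage, then applies GE_MeleeAttack_Damage to the payload's target.
; It then refreshes the target's nameplate and, if the target has a valid controller, its player HUD.
; It prints a debug string and ends, though any failed cast stops the chain before EndAbility.
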(event `self.K2_ActivateAbility`
  (`self.K2_CommitAbility`)
  (bind (_asynctaskproxy _payload) (`AbilityTask_WaitGameplayEvent.WaitGameplayEvent` (struct :`TagName` "Skills.MeleeAttack.DealDamage") null true)
    (:`EventReceived`
      (bind (_eventtag _instigator _target) (break `GameplayEventData` _payload))
      (`self.BP_ApplyGameplayEffectToTarget` (`AbilitySystemBlueprintLibrary.AbilityTargetDataFromActor` _target) "/Game/Power/Abilities/Generic/MeleeAttack/GE_MeleeAttack_Damage.GE_MeleeAttack_Damage_C")
      (bind _aspower_entity (cast `PowerEntity` _target))
      (bind _asbp_nameplate_controller (cast `/Game/Power/UI/NamePlates/BP_NameplateController` (`PowerEntity.NameplateController` _aspower_entity)))
      (bind _asbp_nameplate (cast `/Game/Power/UI/NamePlates/BP_Nameplate` (`WidgetComponent.GetUserWidgetObject` _asbp_nameplate_controller)))
      (`/Game/Power/UI/NamePlates/BP_Nameplate.UpdateNameplate` _asbp_nameplate)
      (bind _returnvalue (`Pawn.GetController` _aspower_entity))
      (`/Engine/EditorBlueprintResources/StandardMacros.IsValid` _returnvalue
        (:`Is Valid`
          (bind _asbp_mmo_player_controller (cast `/Game/Power/Character/Player/BP_MMO_PlayerController` _returnvalue))
          (`/Game/Power/Character/Player/BP_MMO_PlayerController.UpdatePlayerHUD` _asbp_mmo_player_controller))
        (:`Is Not Valid`
          _))
      (`KismetSystemLibrary.PrintString` "Hello")
      (`self.K2_EndAbility`))))