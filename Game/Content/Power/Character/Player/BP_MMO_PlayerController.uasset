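; Player controller giving the player MMO-style mouse and keyboard controls, and creating the status HUD and skillbar widgets.
; Left click targets the PowerEntity under the cursor; holding either button hides the cursor and rotates the camera boom, right also turning the character.
; Axis events drive movement with slower backpedal, both-button forward, turn-or-strafe keys and camera reset behind the character; the wheel zooms.
; Movement axes replicate actor rotation through a server RPC and multicast.
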(event `self.ReceiveBeginPlay`
  ;[0 0.303 1 0.384] Enable PlayerUI
  (bind _returnvalue (`|CreateWidget` "/Game/Power/UI/PlayerUI/BP_PlayerStatusUI.BP_PlayerStatusUI_C"))
  (bind _output_get (set `self.PlayerUI` _returnvalue))
  (`UserWidget.AddToViewport` _output_get 0)
  (`self.UpdatePlayerHUD`)
  (bind _returnvalue_2 (`|CreateWidget` "/Game/Power/UI/PlayerUI/BP_Skillbar.BP_Skillbar_C"))
  (`UserWidget.AddToViewport` _returnvalue_2 0))

(event `InputAction|LeftClick`
  (params (Key :type "Key Structure"))
  ;[1 0.9235 0] Target click
  (:`Pressed`
    (bind _aspower_entity (cast `PowerEntity` (`GameplayStatics.GetPlayerPawn` 0)))
    (bind _aspower_entity_2 (cast `PowerEntity` (`.HitActor` (`GameplayStatics.BreakHitResult` (`self.GetHitResultUnderCursorForObjects` (`GameplayStatics.GetPlayerController` 0) (`|MakeArray` "ObjectTypeQuery3" :!type "EObjectTypeQuery Enum") true))))
      (:`then`
        (`PowerEntity.SetTargetAndHandleCircle` _aspower_entity _aspower_entity_2))
      (:`CastFailed`
        (`PowerEntity.SetTargetAndHandleCircle` _aspower_entity null)))))

(event `InputAction|MouseScrollDown`
  (params (Key :type "Key Structure"))
  ;[0 1 0.7614 0.384] MouseWheel Camera Controls
  (:`Pressed`
    (bind _asbp_mmoplayer (cast `/Game/Power/Character/Player/BP_MMOPlayer` (`GameplayStatics.GetPlayerPawn` 0)))
    (bind _cameraboom (`/Game/Power/Character/Player/BP_MMOPlayer.CameraBoom` _asbp_mmoplayer))
    (set `SpringArmComponent.TargetArmLength` (`KismetMathLibrary.FClamp` (+ (* (`self.ZoomAmount`) (`self.ZoomSensitivity`)) (`SpringArmComponent.TargetArmLength` _cameraboom)) (`self.MinBoomLength`) (`self.MaxBoomLength`)) _cameraboom)))

(event `InputAction|MouseScrollUp`
  (params (Key :type "Key Structure"))
  ;[0 1 0.7614 0.384] MouseWheel Camera Controls
  (:`Pressed`
    (bind _asbp_mmoplayer (cast `/Game/Power/Character/Player/BP_MMOPlayer` (`GameplayStatics.GetPlayerPawn` 0)))
    (bind _cameraboom (`/Game/Power/Character/Player/BP_MMOPlayer.CameraBoom` _asbp_mmoplayer))
    (set `SpringArmComponent.TargetArmLength` (`KismetMathLibrary.FClamp` (- (`SpringArmComponent.TargetArmLength` _cameraboom) (* (`self.ZoomAmount`) (`self.ZoomSensitivity`))) (`self.MinBoomLength`) (`self.MaxBoomLength`)) _cameraboom)))

(event `InputAxis|MoveForward`
  (params (AxisValue :type "Float (single-precision)"))
  ;[0 1 0.7614 0.384] Forward/Backward/Strafe Axis Control
  (`self.AddForwardInput` AxisValue (`KismetMathLibrary.MakeRotator` 0.0 0.0 (.yaw (`self.GetControlRotation`))))
  (set `self.Moving` (or (or (!= AxisValue 0.0) (== (+ (stale `InputAxis|LMBHeld` AxisValue) (stale `InputAxis|RMBHeld` AxisValue)) 2.0)) (!= (stale `InputAxis|StrafeRight` AxisValue) 0.0)) :!label _label)
  ;[1 0.1842 0.254] Update Actor's Rotation Server Side Every Tick
  (`self.UpdateActorPosAndRot` :!label _label_2)
  ;[0 1 0.7614 0.384] If you start moving while LMB isn't held, Reset the Camera Behind the Character
  (if (`self.LeftMousePressed`)
    (set `self.CameraResetting` false)
    (elif (`self.Moving`)
      (set `self.CameraResetting` true))))

(event `Multicast`
  (params (NewRotation :type "Rotator Structure"))
  ;[1 0.1842 0.254] Replicate Actor Rotation and Location To Server
  (`self.K2_SetActorRotation` NewRotation))

(event `InputAxis|StrafeRight`
  (params (AxisValue :type "Float (single-precision)"))
  ;[0 1 0.7614 0.384] Forward/Backward/Strafe Axis Control
  (`self.AddStrafeInput` (`KismetMathLibrary.MakeRotator` 0.0 0.0 (.yaw (`self.GetControlRotation`))) AxisValue)
  (goto _label_2))

(event `Run On Server`
  (params (NewRotation :type "Rotator Structure"))
  ;[1 0.1842 0.254] Replicate Actor Rotation and Location To Server
  (`self.Multicast` NewRotation))

(event `InputAxis|LMBHeld`
  (params (AxisValue :type "Float (single-precision)"))
  ;[0 1 0.7614 0.384] If both LMB and RMB are held, walk forward
  (if (== (+ AxisValue (stale `InputAxis|RMBHeld` AxisValue)) 2.0) :!label _label_3
    (`self.AddForwardInput` 1.0 (`KismetMathLibrary.MakeRotator` 0.0 0.0 (.yaw (`self.GetControlRotation`))))
    (goto _label)))

(event `UpdateActorPosAndRot`
  ;[1 0.1842 0.254] Replicate Actor Rotation and Location To Server
  (bind _asbp_mmoplayer (cast `/Game/Power/Character/Player/BP_MMOPlayer` (`GameplayStatics.GetPlayerPawn` 0)))
  (`/Engine/EditorBlueprintResources/ActorMacros.Switch Has Authority`
    (:`Authority`
      (bind _returnvalue (`self.K2_GetActorRotation` _asbp_mmoplayer))
      (`self.Multicast` _returnvalue))
    (:`Remote`
      (`self.Run On Server` _returnvalue))))

(event `InputAxis|RMBHeld`
  (params (AxisValue :type "Float (single-precision)"))
  ;[0 1 0.7614 0.384] If both LMB and RMB are held, walk forward
  (goto _label_3))

(event `InputAxis|RotateRight`
  (params (AxisValue :type "Float (single-precision)"))
  ;[0 1 0.7614 0.384] Character A/D Rotation
  (if (`self.RightMousePressed`)
    ;[0 1 0.7614 0.384] If right mouse clicked, strafe, don't rotate
    (`self.AddStrafeInput` (`KismetMathLibrary.MakeRotator` 0.0 0.0 (.yaw (`self.GetControlRotation`))) AxisValue)
    (else
      ;[0 1 0.7614 0.384] If LMB held, Rotate Camera and Character
      (if (`self.LeftMousePressed`)
        ;[0 1 0.7614 0.384] If LMB&RMB are not held, rotate character and camera together, if LMB is held then rotate character but not camera
        (bind _asmmo_player (cast `MMO_Player` (`self.K2_GetPawn`) :!label _label_4))
        (`Pawn.AddControllerYawInput` _asmmo_player AxisValue)
        (else
          ;[0 1 0.7614 0.384] Don't Rotate the camera if it is resetting
          (if (and (`self.CameraFreeRotate`) (`self.Moving`))
            (`self.ResetCamera`)
            (goto _label_4)
            (elif (!= AxisValue 0.0)
              (`self.RotateCameraTurn` AxisValue)
              (`self.RotateCharacterToCamera`))))))))

(event `InputAction|RightClick`
  (params (Key :type "Key Structure"))
  ;[0 1 0.7614 0.384] Right Click Handling + UI Control
  (:`Pressed`
    (set `self.RightMousePressed` true)
    (`self.ToggleUIControlOff`)
    ;[0 1 0.7614 0.384] Right clicking snaps the character's rotation to the direction of the camera
    (bind _asbp_mmoplayer (cast `/Game/Power/Character/Player/BP_MMOPlayer` (`GameplayStatics.GetPlayerPawn` 0)))
    (`self.K2_SetActorRotation` (`KismetMathLibrary.MakeRotator` 0.0 0.0 (.yaw (`SceneComponent.RelativeRotation` (`/Game/Power/Character/Player/BP_MMOPlayer.CameraBoom` _asbp_mmoplayer))))))
  (:`Released`
    (set `self.RightMousePressed` false)
    (if (not (`self.leftMousePressed`))
      (`self.ToggleUIControlOn`))))

(event `InputAction|LeftClick`
  (params (Key :type "Key Structure"))
  ;[0 1 0.7614 0.384] Left Click Handling + UI Control
  (:`Pressed`
    (set `self.leftMousePressed` true)
    (`self.ToggleUIControlOff`))
  (:`Released`
    (set `self.leftMousePressed` false)
    (if (not (`self.RightMousePressed`))
      (`self.ToggleUIControlOn`))))

(event `InputAxis|MouseYaw`
  (params (AxisValue :type "Float (single-precision)"))
  (bind _rightmousepressed (`self.RightMousePressed`))
  ;[0 1 0.7614 0.384] Left mouse drag rotates camera, Right Rotates Camera and Character
  (if (or (`self.leftMousePressed`) _rightmousepressed)
    (if _rightmousepressed
      (`self.RotateCharacterToCamera`))
    (`self.RotateCameraTurn` AxisValue)
    (set `self.CameraFreeRotate` true)))

(event `InputAxis|MousePitch`
  (params (AxisValue :type "Float (single-precision)"))
  (bind _rightmousepressed (`self.RightMousePressed`))
  ;[0 1 0.7614 0.384] Left mouse drag rotates camera, Right Rotates Camera and Character
  (if (or (`self.leftMousePressed`) _rightmousepressed)
    (if _rightmousepressed
      (`self.AddPitchInput` AxisValue))
    (`self.RotateCameraPitch` AxisValue)))

(fn `AddForwardInput`
  (params (Value :type "Float (double-precision)") (Rotation :type "Rotator Structure"))
  (bind _returnvalue (`KismetMathLibrary.GetForwardVector` Rotation))
  ;[1 1 1] Forward/Backwards Controls
  (set `self.MovingBackwards` (> -0.1 Value))
  (bind _asbp_mmoplayer (cast `/Game/Power/Character/Player/BP_MMOPlayer` (`GameplayStatics.GetPlayerPawn` 0)))
  (if (`self.MovingBackwards`)
    (`Pawn.AddMovementInput` _asbp_mmoplayer _returnvalue (* Value (`self.BackwardsSpeed`)) false)
    (else
      (`Pawn.AddMovementInput` _asbp_mmoplayer _returnvalue Value false))))

(fn `AddStrafeInput`
  (params (Rotation :type "Rotator Structure") (Value :type "Float (double-precision)"))
  (bind _returnvalue (`KismetMathLibrary.GetRightVector` Rotation))
  ;[1 1 1] Strafing Controls
  (bind _asbp_mmoplayer (cast `/Game/Power/Character/Player/BP_MMOPlayer` (`GameplayStatics.GetPlayerPawn` 0)))
  (if (`self.MovingBackwards`)
    (`Pawn.AddMovementInput` _asbp_mmoplayer _returnvalue (* Value (`self.BackwardsSpeed`)) false)
    (else
      (`Pawn.AddMovementInput` _asbp_mmoplayer _returnvalue Value false))))

(fn `ResetCamera`
  (bind _asbp_mmoplayer (cast `/Game/Power/Character/Player/BP_MMOPlayer` (`GameplayStatics.GetPlayerPawn` 0)))
  (bind _cameraboom (`/Game/Power/Character/Player/BP_MMOPlayer.CameraBoom` _asbp_mmoplayer))
  (bind _pitch (.pitch (`SceneComponent.RelativeRotation` _cameraboom)))
  (bind _yaw (.yaw (`SceneComponent.RelativeRotation` _cameraboom)))
  (bind _yaw_2 (.yaw (`SceneComponent.K2_GetComponentRotation` (`Actor.RootComponent` _asbp_mmoplayer))))
  (if (== _yaw _yaw_2)
    (set `self.CameraResetting` false)
    (else
      (`SceneComponent.K2_SetRelativeRotation` _cameraboom (`KismetMathLibrary.RInterpTo_Constant` (`KismetMathLibrary.MakeRotator` 0.0 _pitch _yaw) (`KismetMathLibrary.MakeRotator` 0.0 _pitch _yaw_2) (`GameplayStatics.GetWorldDeltaSeconds`) 200.0) false false))))

(fn `RotateCameraPitch`
  (params (Value :type "Float (double-precision)"))
  (bind _playercameramanager (`self.PlayerCameraManager`))
  ;[1 1 1] Rotate the camera with the LookUp axis input (pitch)
  (bind _asbp_mmoplayer (cast `/Game/Power/Character/Player/BP_MMOPlayer` (`GameplayStatics.GetPlayerPawn` 0)))
  (bind _cameraboom (`/Game/Power/Character/Player/BP_MMOPlayer.CameraBoom` _asbp_mmoplayer))
  (`SceneComponent.K2_SetWorldRotation` _cameraboom (`KismetMathLibrary.MakeRotator` 0.0 (`KismetMathLibrary.FClamp` (+ (* Value (`self.InputPitchScale`)) (.pitch (`SceneComponent.K2_GetComponentRotation` _cameraboom))) (`PlayerCameraManager.ViewPitchMin` _playercameramanager) (`PlayerCameraManager.ViewPitchMax` _playercameramanager)) (.yaw (`SceneComponent.K2_GetComponentRotation` _cameraboom))) false false))

(fn `RotateCameraTurn`
  (params (Value :type "Float (double-precision)"))
  ;[1 1 1] Rotate Camera with the turn axis input
  (bind _asbp_mmoplayer (cast `/Game/Power/Character/Player/BP_MMOPlayer` (`GameplayStatics.GetPlayerPawn` 0)))
  (bind _cameraboom (`/Game/Power/Character/Player/BP_MMOPlayer.CameraBoom` _asbp_mmoplayer))
  (`SceneComponent.K2_SetWorldRotation` _cameraboom (`KismetMathLibrary.MakeRotator` 0.0 (.pitch (`SceneComponent.K2_GetComponentRotation` _cameraboom)) (+ (* Value (`self.CameraRotateModifier`)) (.yaw (`SceneComponent.K2_GetComponentRotation` _cameraboom)))) false false))

(fn `RotateCharacterToCamera`
  (bind _asbp_mmoplayer (cast `/Game/Power/Character/Player/BP_MMOPlayer` (`GameplayStatics.GetPlayerPawn` 0)))
  (`self.SetControlRotation` (`KismetMathLibrary.MakeRotator` 0.0 0.0 (.yaw (`SceneComponent.RelativeRotation` (`/Game/Power/Character/Player/BP_MMOPlayer.CameraBoom` _asbp_mmoplayer))))))

(fn `ToggleUIControlOff`
  (bind _returnvalue (`GameplayStatics.GetPlayerController` 0))
  (`WidgetBlueprintLibrary.SetInputMode_GameOnly` _returnvalue)
  (set `PlayerController.bShowMouseCursor` false _returnvalue)
  (set `PlayerController.bEnableMouseOverEvents` false _returnvalue)
  (set `PlayerController.bEnableClickEvents` false _returnvalue))

(fn `ToggleUIControlON`
  (bind _returnvalue (`GameplayStatics.GetPlayerController` 0))
  (`WidgetBlueprintLibrary.SetInputMode_GameAndUIEx` _returnvalue null)
  (set `PlayerController.bShowMouseCursor` true _returnvalue)
  (set `PlayerController.bEnableMouseOverEvents` true _returnvalue)
  (set `PlayerController.bEnableClickEvents` true _returnvalue))

(fn `UpdatePlayerHUD`
  (bind _aspower_entity (cast `PowerEntity` (`self.K2_GetPawn`)))
  (bind _asbp_player_status_ui (cast `/Game/Power/UI/PlayerUI/BP_PlayerStatusUI` (`self.PlayerUI`)))
  (bind _returnvalue (`PowerEntity.GetHealth` _aspower_entity))
  (bind _returnvalue_2 (`PowerEntity.GetMaxHealth` _aspower_entity))
  (`/Game/Power/UI/PlayerUI/BP_PlayerStatusUI.UpdateWidgetValues` _asbp_player_status_ui (`PowerEntity.Name` _aspower_entity) (`PowerEntity.Level` _aspower_entity) _returnvalue _returnvalue_2 (`PowerEntity.Mana` _aspower_entity) (`PowerEntity.MaxMana` _aspower_entity)))

(fn `UserConstructionScript`)